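; Short-lived Chaos Emeralds effect actor that shows seven colored emeralds, switches them to a transform material, then destroys itself.
; On BeginPlay, after a brief delay, it gives each emerald component its color material and attaches a matching particle system.
; A second delay leads to the shared material swap, and a final short delay precedes destruction.
; Delays scale by global time dilation, keeping the timing constant in real time.
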(event `self.ReceiveBeginPlay`
  (bind _red (`self.red`))
  (bind _blue (`self.blue`))
  (bind _yellow (`self.yellow`))
  (bind _green (`self.green`))
  (bind _purple (`self.purple`))
  (bind _grey (`self.grey`))
  (`KismetSystemLibrary.Delay` (* 0.2 (`GameplayStatics.GetGlobalTimeDilation`)))
  (`|ExecutionSequence`
    (:`then_0`
      (`PrimitiveComponent.SetMaterial` _red 0 "/Game/Objects/Assets/ChaosEmerald/EmeraldMAT.EmeraldMAT"))
    (:`then_1`
      (`PrimitiveComponent.SetMaterial` _blue 0 "/Game/Objects/Assets/ChaosEmerald/EmeraldMAT_DarkBlue.EmeraldMAT_DarkBlue"))
    (:`then_2`
      (`PrimitiveComponent.SetMaterial` _yellow 0 "/Game/Objects/Assets/ChaosEmerald/EmeraldMAT_Yellow.EmeraldMAT_Yellow"))
    (:`then_3`
      (`PrimitiveComponent.SetMaterial` _green 0 "/Game/Objects/Assets/ChaosEmerald/EmeraldMAT_Green.EmeraldMAT_Green"))
    (:`then_4`
      (`PrimitiveComponent.SetMaterial` _purple 0 "/Game/Objects/Assets/ChaosEmerald/EmeraldMAT_Blue.EmeraldMAT_Blue")
      (`PrimitiveComponent.SetMaterial` (`self.turquois`) 0 "/Game/Objects/Assets/ChaosEmerald/EmeraldMAT_Blue.EmeraldMAT_Blue"))
    (:`then_5`
      (`PrimitiveComponent.SetMaterial` _purple 0 "/Game/Objects/Assets/ChaosEmerald/EmeraldMAT_Purple.EmeraldMAT_Purple"))
    (:`then_6`
      (`PrimitiveComponent.SetMaterial` _grey 0 "/Game/Objects/Assets/ChaosEmerald/EmeraldMAT_Silver.EmeraldMAT_Silver"))
    (:`then_7`
      (`KismetSystemLibrary.Delay` (* 1.0 (`GameplayStatics.GetGlobalTimeDilation`)))
      (`|ExecutionSequence`
        (:`then_0`
          (`PrimitiveComponent.SetMaterial` _red 0 "/Game/Blueprints/transformmaterial.transformmaterial"))
        (:`then_1`
          (`PrimitiveComponent.SetMaterial` _blue 0 "/Game/Blueprints/transformmaterial.transformmaterial"))
        (:`then_2`
          (`PrimitiveComponent.SetMaterial` _yellow 0 "/Game/Blueprints/transformmaterial.transformmaterial"))
        (:`then_3`
          (`PrimitiveComponent.SetMaterial` _green 0 "/Game/Blueprints/transformmaterial.transformmaterial"))
        (:`then_4`
          (`PrimitiveComponent.SetMaterial` (`self.turquois`) 0 "/Game/Blueprints/transformmaterial.transformmaterial"))
        (:`then_5`
          (`PrimitiveComponent.SetMaterial` _purple 0 "/Game/Blueprints/transformmaterial.transformmaterial"))
        (:`then_6`
          (`PrimitiveComponent.SetMaterial` _grey 0 "/Game/Blueprints/transformmaterial.transformmaterial"))
        (:`then_7`
          (`KismetSystemLibrary.Delay` (* 0.2 (`GameplayStatics.GetGlobalTimeDilation`)))
          (`self.K2_DestroyActor`))))
    (:`then_8`
      (`NiagaraFunctionLibrary.SpawnSystemAttached` "/Game/Particles/red.red" (`self.red`) "None" (0.0 0.0 0.0) (struct) "KeepRelativeOffset"))
    (:`then_9`
      (`NiagaraFunctionLibrary.SpawnSystemAttached` "/Game/Particles/blue.blue" (`self.blue`) "None" (0.0 0.0 0.0) (struct) "KeepRelativeOffset"))
    (:`then_10`
      (`NiagaraFunctionLibrary.SpawnSystemAttached` "/Game/Particles/yellow.yellow" (`self.yellow`) "None" (0.0 0.0 0.0) (struct) "KeepRelativeOffset"))
    (:`then_11`
      (`NiagaraFunctionLibrary.SpawnSystemAttached` "/Game/Particles/green.green" (`self.green`) "None" (0.0 0.0 0.0) (struct) "KeepRelativeOffset"))
    (:`then_12`
      (`NiagaraFunctionLibrary.SpawnSystemAttached` "/Game/Particles/turquoise.turquoise" (`self.turquois`) "None" (0.0 0.0 0.0) (struct) "KeepRelativeOffset"))
    (:`then_13`
      (`NiagaraFunctionLibrary.SpawnSystemAttached` "/Game/Particles/purple.purple" (`self.purple`) "None" (0.0 0.0 0.0) (struct) "KeepRelativeOffset"))
    (:`then_14`
      (`NiagaraFunctionLibrary.SpawnSystemAttached` "/Game/Particles/grey.grey" (`self.grey`) "None" (0.0 0.0 0.0) (struct) "KeepRelativeOffset"))))

(fn `UserConstructionScript`)