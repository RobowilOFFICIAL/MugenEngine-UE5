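; ShadowTargetActor is a target marker for the Shadow character that animates on spawn and always faces the player camera.
; On BeginPlay, three staggered timelines scale Target2, Target3 and Target4 relative to the actor's scale, creating a rippling sequence.
; Every Tick it billboards by rotating toward the player camera's location.
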(event `self.ReceiveBeginPlay`
  (bind _returnvalue (`self.GetActorScale3D`))
  (`|ExecutionSequence`
    (:`then_0`
      (bind (_direction _newtrack_0) (`Timeline|Timeline_0` :!via `PlayFromStart`)
        (:`Update`
          (`SceneComponent.SetWorldScale3D` (`self.Target2`) (* _returnvalue (`KismetMathLibrary.MakeVector` _newtrack_0 _newtrack_0 _newtrack_0))))))
    (:`then_1`
      (`KismetSystemLibrary.Delay` 0.075)
      (bind (_direction_2 _newtrack_0_2) (`Timeline|Timeline_1` :!via `PlayFromStart`)
        (:`Update`
          (`SceneComponent.SetWorldScale3D` (`self.Target3`) (* _returnvalue (`KismetMathLibrary.MakeVector` _newtrack_0_2 _newtrack_0_2 _newtrack_0_2))))))
    (:`then_2`
      (`KismetSystemLibrary.Delay` 0.15)
      (bind (_direction_3 _newtrack_0_3) (`Timeline|Timeline_2` :!via `PlayFromStart`)
        (:`Update`
          (`SceneComponent.SetWorldScale3D` (`self.Target4`) (* _returnvalue (`KismetMathLibrary.MakeVector` _newtrack_0_3 _newtrack_0_3 _newtrack_0_3))))))))

(event `self.ReceiveTick`
  (params (DeltaSeconds :type "Float (single-precision)"))
  (`self.K2_SetActorRotation` (`KismetMathLibrary.FindLookAtRotation` (`self.K2_GetActorLocation`) (`PlayerCameraManager.GetCameraLocation` (`GameplayStatics.GetPlayerCameraManager` 0)))))

(fn `UserConstructionScript`)